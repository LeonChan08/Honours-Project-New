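; Rocks is a Blueprint for a physics rock that varies its size, mass and starting motion on BeginPlay.
; It picks a random uniform scale for the Rock component and overrides its mass in proportion to that scale.
; It then applies one random impulse value to both X and Y, so the push runs along a single horizontal diagonal in either direction.
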(event `self.ReceiveBeginPlay`
  (bind _rock (`self.Rock`))
  ;[1 1 1] Set rock size and mass
  (bind _output_get (set `self.RockSize` (`KismetMathLibrary.RandomFloatInRange` 0.2 2.0)))
  (`SceneComponent.SetWorldScale3D` _rock (`KismetMathLibrary.Conv_DoubleToVector` _output_get))
  (`PrimitiveComponent.SetMassOverrideInKg` _rock "None" (* _output_get 1.5) true)
  ;[1 1 1] Make rocks move in random direction
  (bind _output_get_2 (set `self.RockImpulse` (`KismetMathLibrary.RandomFloatInRange` -250.0 250.0)))
  (`PrimitiveComponent.AddImpulse` (`self.Rock`) (`KismetMathLibrary.MakeVector` _output_get_2 _output_get_2) "None" false))

(fn `UserConstructionScript`)