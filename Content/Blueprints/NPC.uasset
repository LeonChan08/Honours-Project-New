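; NPC actor that offers multi-line chat dialogue when the player enters its trigger box.
; Overlap shows the highlight marker and the player's touch dialogue button and creates the chat widget; leaving reverses this.
; EventDialogueOccurs passes NPCText to the widget and advances its row through a resettable DoOnce.
; After the last line it removes the widget and restores the player's walking movement.
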(event `self.NPC_Chat_Triggerbox.OnComponentBeginOverlap`
  (params (OverlappedComponent :type "PrimitiveComponent Object Reference") (OtherActor :type "Actor Object Reference") (OtherComp :type "PrimitiveComponent Object Reference") (OtherBodyIndex :type Integer) (bFromSweep :type Boolean) (SweepResult :type "HitResult Structure (by ref)"))
  ;[1 1 1] Highlight the NPC in green when overlapped/reverse it on end
  (bind _asthird_person_character (cast `/Game/Blueprints/ThirdPersonCharacter` OtherActor))
  (`SceneComponent.SetVisibility` (`self.Highlight_Marker`) true false)
  (`Widget.SetVisibility` (`/Game/Blueprints/UI/Main_Game_UI_AndTouch.Right_Touch_Button_Dialogue` (`/Game/Blueprints/ThirdPersonCharacter.MainGameUIAndRightTouch_Ref` _asthird_person_character)) "Visible")
  ;[1 1 1] Add dialogue UI
  (bind _returnvalue (`|CreateWidget` "/Game/Blueprints/UI/Chat_Widget_BP.Chat_Widget_BP_C"))
  (bind _output_get (set `self.DialogueUI` _returnvalue))
  (`UserWidget.AddToViewport` _output_get 0))

(event `self.NPC_Chat_Triggerbox.OnComponentEndOverlap`
  (params (OverlappedComponent :type "PrimitiveComponent Object Reference") (OtherActor :type "Actor Object Reference") (OtherComp :type "PrimitiveComponent Object Reference") (OtherBodyIndex :type Integer))
  (bind _dialogueui (`self.DialogueUI`))
  ;[1 1 1] Highlight the NPC in green when overlapped/reverse it on end
  (bind _asthird_person_character (cast `/Game/Blueprints/ThirdPersonCharacter` OtherActor))
  (`SceneComponent.SetVisibility` (`self.Highlight_Marker`) false false)
  (`Widget.SetVisibility` (`/Game/Blueprints/UI/Main_Game_UI_AndTouch.Right_Touch_Button_Dialogue` (`/Game/Blueprints/ThirdPersonCharacter.MainGameUIAndRightTouch_Ref` _asthird_person_character)) "Hidden")
  ;[1 1 1] Remove dialogue UI
  (`/Engine/EditorBlueprintResources/StandardMacros.IsValid` _dialogueui
    (:`Is Valid`
      (`Widget.RemoveFromParent` _dialogueui))))

(event `/Game/Blueprints/DialogueInterface.event_Dialogue_Occurs`
  (bind _dialogueui (`self.DialogueUI`))
  (bind _returnvalue (+ (`/Game/Blueprints/UI/Chat_Widget_BP.textrow` (`self.DialogueUI`)) 1))
  ;[1 1 1] If there is an event, reset the dialogue (if reset is called), set the text, have UI appear
  (`/Engine/EditorBlueprintResources/StandardMacros.DoOnce` false :!label _label
    (:`Completed`
      (set `/Game/Blueprints/UI/Chat_Widget_BP.text` (`self.NPC Text`) _dialogueui)
      (`Widget.SetVisibility` (`/Game/Blueprints/UI/Chat_Widget_BP.TextBoxBackground` _dialogueui) "Visible")
      (`Widget.SetVisibility` (`/Game/Blueprints/UI/Chat_Widget_BP.TextInsideBox` _dialogueui) "Visible")
      ;[1 1 1] If true, remove dialogue UI. If false, display the next line.
      (if (> _returnvalue (- (`KismetArrayLibrary.Array_Length` (`self.NPC Text`)) 1))
        (`Widget.RemoveFromParent` (`self.DialogueUI`))
        (`self.resetDialogue`)
        ;[1 1 1] Allow player to move again
        (`CharacterMovementComponent.SetMovementMode` (`Character.CharacterMovement` (`GameplayStatics.GetPlayerCharacter` 0)) "MOVE_Walking" 0)
        (else
          (set `/Game/Blueprints/UI/Chat_Widget_BP.textrow` _returnvalue (`self.DialogueUI`))
          (`self.resetDialogue`))))))

(event `resetDialogue`
  ;[1 1 1] If there is an event, reset the dialogue (if reset is called), set the text, have UI appear
  (goto _label :!via `Reset`))

(fn `UserConstructionScript`)