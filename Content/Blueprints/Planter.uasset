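; Planter actor where the player spends a seed to grow a plant, then harvests a random plant type into the inventory.
; Its hitbox overlap toggles touch UI and highlight and binds the seed button, which plants, harvests or shows a warning.
; A Timeline drives growth, feeds the world timer widget through the game instance and polls a points-used flag for speed-ups.
; Harvesting increments the game instance's inventory and total arrays.
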(event `self.ReceiveBeginPlay`
  (bind _asinventory_data_game_instance_bp (cast `/Game/Blueprints/InventoryData_GameInstance_BP` (`GameplayStatics.GetGameInstance`)))
  (set `self.As Inventory Data Game Instance BP` _asinventory_data_game_instance_bp)
  (set `self.PlanterHitboxLocation` (`SceneComponent.K2_GetComponentLocation` (`self.PlanterHitbox`))))

(event `self.PlanterHitbox.OnComponentBeginOverlap`
  (params (OverlappedComponent :type "PrimitiveComponent Object Reference") (OtherActor :type "Actor Object Reference") (OtherComp :type "PrimitiveComponent Object Reference") (OtherBodyIndex :type Integer) (bFromSweep :type Boolean) (SweepResult :type "HitResult Structure (by ref)"))
  (bind _in_world_widget (`self.In_World_Widget`))
  (bind _main_game_uiand_right_touch_ref (`self.Main Game UIAnd Right Touch Ref`))
  ;[1 1 1] Make interactable hitbox touchable, hide dialogue hitbox, show interaction screen canvas
  (bind _asthird_person_character (cast `/Game/Blueprints/ThirdPersonCharacter` OtherActor))
  (bind _output_get (set `self.Main Game UIAnd Right Touch Ref` (`/Game/Blueprints/ThirdPersonCharacter.MainGameUIAndRightTouch_Ref` _asthird_person_character)))
  (`Widget.SetVisibility` (`/Game/Blueprints/UI/Main_Game_UI_AndTouch.Right_Touch_Button_Dialogue` _output_get) "Hidden")
  (`Widget.SetVisibility` (`/Game/Blueprints/UI/Main_Game_UI_AndTouch.Right_Touch_Button_Interactables_Eggs` _output_get) "Hidden")
  (bind _right_touch_button_interactable_seeds (`/Game/Blueprints/UI/Main_Game_UI_AndTouch.Right_Touch_Button_Interactable_Seeds` _output_get))
  (`Widget.SetVisibility` _right_touch_button_interactable_seeds "Visible")
  (`Widget.SetVisibility` (`/Game/Blueprints/UI/Main_Game_UI_AndTouch.Seed_Screen_Canvas_1` _output_get) "Visible")
  (add `Button.OnClicked` _right_touch_button_interactable_seeds (delegate `OnClicked_Event_Interactable`))
  (if (`self.Seedplanted`)
    (if (`SceneComponent.IsVisible` (`self.Plant`))
      (`SceneComponent.SetVisibility` (`self.Highlight`) true false :!label _label)
      (else
        ;[0.5541 1 0.6092] Start timer, tell the player a seed is planted, and display the timer above the planter
        (if (not (`SceneComponent.IsVisible` _in_world_widget))
          (`SceneComponent.SetVisibility` _in_world_widget true false :!label _label_2)
          (`Widget.SetVisibility` (`/Game/Blueprints/UI/Main_Game_UI_AndTouch.Seedhorizontalbox_1` (`self.Main Game UIAnd Right Touch Ref`)) "Visible")
          (`Widget.SetVisibility` (`/Game/Blueprints/UI/Main_Game_UI_AndTouch.Speed_up_button` (`self.Main Game UIAnd Right Touch Ref`)) "Visible")
          (`SceneComponent.SetVisibility` (`self.Highlight`) false false)
          (`Widget.SetVisibility` (`/Game/Blueprints/UI/Main_Game_UI_AndTouch.Seedhorizontalbox_1` (`self.Main Game UIAnd Right Touch Ref`)) "Hidden")
          (bind (_direction _plant_track) (`Timeline|PlantTimer` :`NewTime` 599.900024 :!via `PlayFromStart` :!label _label_3)
            (:`Update`
              ;;[1 1 1] Used for the world UI timer
              (set `/Game/Blueprints/InventoryData_GameInstance_BP.Plant_Timer` _plant_track (`self.As Inventory Data Game Instance BP`))
              ;;[1 1 1] Every tick check if the points used boolean is true. if it is, set it to false, set the timer to end. (Using points to speed up growth).
              (if (`/Game/Blueprints/UI/Main_Game_UI_AndTouch.Points_Used` _main_game_uiand_right_touch_ref)
                (set `/Game/Blueprints/UI/Main_Game_UI_AndTouch.Points_Used` false _main_game_uiand_right_touch_ref)
                (set `/Game/Blueprints/InventoryData_GameInstance_BP.Is_Plant_Ready` true (`self.As Inventory Data Game Instance BP`))
                (goto _label_3 :!via `SetNewTime`)))
            (:`Finished`
              (set `/Game/Blueprints/InventoryData_GameInstance_BP.Is_Plant_Ready` true (`self.As Inventory Data Game Instance BP`))
              (`SceneComponent.SetVisibility` (`self.Plant`) true false)
              (`SceneComponent.SetVisibility` (`self.In_World_Widget`) false false)
              (`Widget.SetVisibility` (`/Game/Blueprints/UI/Main_Game_UI_AndTouch.Speed_up_button` (`self.Main Game UIAnd Right Touch Ref`)) "Hidden"))))))
    (else
      (goto _label))))

(event `OnClicked_Event_Interactable`
  (bind _as_inventory_data_game_instance_bp (`self.As Inventory Data Game Instance BP`))
  (bind _rng (`self.RNG`))
  (bind _no_seeds_text (`/Game/Blueprints/UI/Main_Game_UI_AndTouch.No_Seeds_Text` (`self.Main Game UIAnd Right Touch Ref`)))
  (bind _seed_already_planted_text (`/Game/Blueprints/UI/Main_Game_UI_AndTouch.Seed_Already_Planted_Text` (`self.Main Game UIAnd Right Touch Ref`)))
  (bind _seeds (`/Game/Blueprints/InventoryData_GameInstance_BP.Seeds` _as_inventory_data_game_instance_bp))
  ;[0.3984 1 0.3524] Player clicks when inside hitbox
  (if (`self.Seedplanted`)
    ;[0.2956 0.5492 1] If plant has grown, set it to invisible and add it to inventory, set seed planted to false
    (if (`SceneComponent.IsVisible` (`self.Plant`))
      (`SceneComponent.SetVisibility` (`self.Plant`) false false)
      (set `self.Seedplanted` false)
      (set `/Game/Blueprints/InventoryData_GameInstance_BP.Is_Plant_Ready` false (`self.As Inventory Data Game Instance BP`))
      ;[0.2891 0.3963 1] Two arrays are stored in InventoryData. A random number is called and stored in RNG. That number is used to get the inventory index of the int plant array. It is then set as its current value +1.
      (bind _asinventory_data_game_instance_bp (cast `/Game/Blueprints/InventoryData_GameInstance_BP` (`GameplayStatics.GetGameInstance`)))
      (bind _output_get (set `self.RNG` (`KismetMathLibrary.RandomIntegerInRange` 0 4)))
      (bind _plants_inventory_total (`/Game/Blueprints/InventoryData_GameInstance_BP.Plants_Inventory_Total` _asinventory_data_game_instance_bp))
      (bind _result (`/Engine/EditorBlueprintResources/StandardMacros.IncrementInt` (`|GetArrayItem` _plants_inventory_total _output_get))
        (:`  `
          (`KismetArrayLibrary.Array_Set` _plants_inventory_total _rng _result)
          (bind _plants_inventory (`/Game/Blueprints/InventoryData_GameInstance_BP.Plants_Inventory` _asinventory_data_game_instance_bp))
          (bind _result_2 (`/Engine/EditorBlueprintResources/StandardMacros.IncrementInt` (`|GetArrayItem` _plants_inventory _output_get))
            (:`  `
              (`KismetArrayLibrary.Array_Set` _plants_inventory _rng _result_2)
              ;;[0.9522 0.3821 1] The same RNG is used to get the name of the mineral in the mineral string array (holds the mineral names).
              (set `/Game/Blueprints/InventoryData_GameInstance_BP.Plant_Grown` (`|GetArrayItem` (`/Game/Blueprints/InventoryData_GameInstance_BP.Plants` _asinventory_data_game_instance_bp) (`self.RNG`)) (`self.As Inventory Data Game Instance BP`))
              (`Widget.SetVisibility` (`/Game/Blueprints/UI/Main_Game_UI_AndTouch.Plant_Type_Text_1` (`self.Main Game UIAnd Right Touch Ref`)) "Visible")
              (`KismetSystemLibrary.Delay` 3.0)
              (`Widget.SetVisibility` (`/Game/Blueprints/UI/Main_Game_UI_AndTouch.Plant_Type_Text_1` (`self.Main Game UIAnd Right Touch Ref`)) "Hidden")))))
      (else
        ;[1 0 0] Tells player they have already planted a seed here
        (`Widget.SetVisibility` _seed_already_planted_text "Visible")
        (`KismetSystemLibrary.Delay` 3.0)
        (`Widget.SetVisibility` _seed_already_planted_text "Hidden")))
    (else
      ;[0.3146 1 0.4649] If player has seed in inventory, remove one, set seed to planted
      (if (> _seeds 0)
        (set `/Game/Blueprints/InventoryData_GameInstance_BP.Seeds` (- _seeds 1) _as_inventory_data_game_instance_bp)
        (set `self.Seedplanted` true)
        (goto _label_2)
        (else
          ;[1 0 0] Tells player they have no seeds to plant
          (`Widget.SetVisibility` _no_seeds_text "Visible")
          (`KismetSystemLibrary.Delay` 3.0)
          (`Widget.SetVisibility` _no_seeds_text "Hidden"))))))

(event `self.PlanterHitbox.OnComponentEndOverlap`
  (params (OverlappedComponent :type "PrimitiveComponent Object Reference") (OtherActor :type "Actor Object Reference") (OtherComp :type "PrimitiveComponent Object Reference") (OtherBodyIndex :type Integer))
  ;[1 1 1] Make dialogue hitbox touchable, hide interactable hitbox
  (bind _asthird_person_character (cast `/Game/Blueprints/ThirdPersonCharacter` OtherActor))
  (`Widget.SetVisibility` (`/Game/Blueprints/UI/Main_Game_UI_AndTouch.Right_Touch_Button_Interactable_Seeds` (`/Game/Blueprints/ThirdPersonCharacter.MainGameUIAndRightTouch_Ref` _asthird_person_character)) "Hidden")
  (`Widget.SetVisibility` (`/Game/Blueprints/UI/Main_Game_UI_AndTouch.Seed_Screen_Canvas_1` (`self.Main Game UIAnd Right Touch Ref`)) "Hidden")
  (`SceneComponent.SetVisibility` (`self.Highlight`) false false))

(fn `UserConstructionScript`)