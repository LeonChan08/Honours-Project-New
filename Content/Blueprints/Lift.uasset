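; Lift actor that carries the third-person character between a start (bottom) and end (top) position.
; A timeline lerps the platform's relative location, playing toward the end and reversing toward the start.
; Overlapping the lift trigger sends it to the opposite end, while lower and upper landing triggers call it to their level.
; The landing checks compare world location to positions that are otherwise used as relative.
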(event `self.ReceiveBeginPlay`
  (bind _lift_platform (`self.Lift_Platform`))
  ;[1 1 1] Set lift location
  (`SceneComponent.K2_SetRelativeLocation` _lift_platform (`SceneComponent.RelativeLocation` _lift_platform) false false))

(event `self.Trigger.OnComponentBeginOverlap`
  (params (OverlappedComponent :type "PrimitiveComponent Object Reference") (OtherActor :type "Actor Object Reference") (OtherComp :type "PrimitiveComponent Object Reference") (OtherBodyIndex :type Integer) (bFromSweep :type Boolean) (SweepResult :type "HitResult Structure (by ref)"))
  ;[1 1 1] When player steps in lift, check if its at top or bottom and move to opposite location
  (cast `/Game/Blueprints/ThirdPersonCharacter` OtherActor)
  (if (== (`SceneComponent.RelativeLocation` (`self.Lift_Platform`)) (`self.Start_Position`))
    ;[1 1 1] Move Platform up or down
    (bind (_direction _lift_timeline) (`Timeline|Lift_Timeline` :!label _label)
      (:`Update`
        (`SceneComponent.K2_SetRelativeLocation` (`self.Lift_Platform`) (`KismetMathLibrary.VLerp` (`self.Start_Position`) (`self.End_Position`) _lift_timeline) false false)))
    (else
      (goto _label :!via `Reverse`))))

(event `self.Lower_platform_Trigger.OnComponentBeginOverlap`
  (params (OverlappedComponent :type "PrimitiveComponent Object Reference") (OtherActor :type "Actor Object Reference") (OtherComp :type "PrimitiveComponent Object Reference") (OtherBodyIndex :type Integer) (bFromSweep :type Boolean) (SweepResult :type "HitResult Structure (by ref)"))
  ;[1 1 1] Call for lift at bottom
  (cast `/Game/Blueprints/ThirdPersonCharacter` OtherActor)
  (if (`KismetMathLibrary.NotEqualExactly_VectorVector` (`SceneComponent.K2_GetComponentLocation` (`self.Lift_Platform`)) (`self.Start_Position`))
    (goto _label :!via `Reverse`)))

(event `self.Upper_platform_Trigger.OnComponentBeginOverlap`
  (params (OverlappedComponent :type "PrimitiveComponent Object Reference") (OtherActor :type "Actor Object Reference") (OtherComp :type "PrimitiveComponent Object Reference") (OtherBodyIndex :type Integer) (bFromSweep :type Boolean) (SweepResult :type "HitResult Structure (by ref)"))
  ;[1 1 1] Call for lift at top
  (cast `/Game/Blueprints/ThirdPersonCharacter` OtherActor)
  (if (`KismetMathLibrary.NotEqualExactly_VectorVector` (`SceneComponent.K2_GetComponentLocation` (`self.Lift_Platform`)) (`self.End_Position`))
    (goto _label)))

(fn `UserConstructionScript`)