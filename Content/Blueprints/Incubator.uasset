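; Incubator actor where the player turns an egg from inventory into a random creature after a timed wait.
; Entering its hitbox shows egg UI and binds the touch button, which starts incubation, collects the hatched creature, or flashes an in-use or no-eggs message.
; A timeline writes progress to the inventory GameInstance and can be cut short by a points-based speed-up.
; When it finishes, exclamation marks flag the egg as ready.
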(event `self.ReceiveBeginPlay`
  (bind _asinventory_data_game_instance_bp (cast `/Game/Blueprints/InventoryData_GameInstance_BP` (`GameplayStatics.GetGameInstance`)))
  (set `self.As Inventory Data Game Instance BP` _asinventory_data_game_instance_bp))

(event `self.IncubatorHitbox.OnComponentBeginOverlap`
  (params (OverlappedComponent :type "PrimitiveComponent Object Reference") (OtherActor :type "Actor Object Reference") (OtherComp :type "PrimitiveComponent Object Reference") (OtherBodyIndex :type Integer) (bFromSweep :type Boolean) (SweepResult :type "HitResult Structure (by ref)"))
  ;[1 1 1] Make interactable hitbox touchable, hide dialogue hitbox, show interaction screen canvas
  (bind _asthird_person_character (cast `/Game/Blueprints/ThirdPersonCharacter` OtherActor))
  (bind _output_get (set `self.Main Game UIAnd Right Touch Ref` (`/Game/Blueprints/ThirdPersonCharacter.MainGameUIAndRightTouch_Ref` _asthird_person_character)))
  (`Widget.SetVisibility` (`/Game/Blueprints/UI/Main_Game_UI_AndTouch.Right_Touch_Button_Dialogue` _output_get) "Hidden")
  (`Widget.SetVisibility` (`/Game/Blueprints/UI/Main_Game_UI_AndTouch.Right_Touch_Button_Interactable_Seeds` _output_get) "Hidden")
  (`Widget.SetVisibility` (`/Game/Blueprints/UI/Main_Game_UI_AndTouch.Eggs_Screen_Canvas` _output_get) "Visible")
  (`Widget.SetVisibility` (`/Game/Blueprints/UI/Main_Game_UI_AndTouch.Right_Touch_Button_Interactables_Eggs` _output_get) "Visible")
  (add `Button.OnClicked` (`/Game/Blueprints/UI/Main_Game_UI_AndTouch.Right_Touch_Button_Interactables_Eggs` _output_get) (delegate `OnClicked_Event_Interactable`))
  (if (`self.EggIncubated`)
    (if (`SceneComponent.IsVisible` (`self.Exclamation mark`))
      (`SceneComponent.SetVisibility` (`self.Highlight`) true false :!label _label))
    (else
      (goto _label))))

(event `OnClicked_Event_Interactable`
  (bind _main_game_uiand_right_touch_ref (`self.Main Game UIAnd Right Touch Ref`))
  (bind _as_inventory_data_game_instance_bp (`self.As Inventory Data Game Instance BP`))
  (bind _in_world_widget (`self.In_World_Widget`))
  (bind _no_eggs_text (`/Game/Blueprints/UI/Main_Game_UI_AndTouch.No_Eggs_Text` (`self.Main Game UIAnd Right Touch Ref`)))
  (bind _incubator_in_use_text (`/Game/Blueprints/UI/Main_Game_UI_AndTouch.Incubator_In_Use_Text` (`self.Main Game UIAnd Right Touch Ref`)))
  ;[0.3984 1 0.3524] Player clicks when inside hitbox
  (if (`self.EggIncubated`)
    ;[0.2956 0.5492 1] If egg is finished incubating, remove exclamation mark, and add it to inventory, set egg incubated to false
    (if (`SceneComponent.IsVisible` (`self.Exclamation mark`))
      (`SceneComponent.SetVisibility` (`self.Exclamation mark`) false false)
      (`SceneComponent.SetVisibility` (`self.Exclamation mark1`) false false)
      (set `self.EggIncubated` false)
      (`SceneComponent.SetVisibility` (`self.Egg`) false false)
      (set `/Game/Blueprints/InventoryData_GameInstance_BP.Is_Egg_Ready` false (`self.As Inventory Data Game Instance BP`))
      ;[0.2891 0.3963 1] Two arrays are stored in InventoryData. A random number is called and stored in RNG. That number is used to get the inventory index of the int egg creature array. It is then set as its current value +1.
      (bind _asinventory_data_game_instance_bp (cast `/Game/Blueprints/InventoryData_GameInstance_BP` (`GameplayStatics.GetGameInstance`)))
      (bind _output_get (set `self.RNG` (`KismetMathLibrary.RandomIntegerInRange` 0 4)))
      (bind _egg_creature_inventory_total (`/Game/Blueprints/InventoryData_GameInstance_BP.Egg_Creature_Inventory_Total` _asinventory_data_game_instance_bp))
      (bind _result (`/Engine/EditorBlueprintResources/StandardMacros.IncrementInt` (`|GetArrayItem` _egg_creature_inventory_total _output_get))
        (:`  `
          (`KismetArrayLibrary.Array_Set` _egg_creature_inventory_total (`self.RNG`) _result)
          (bind _egg_creature_inventory (`/Game/Blueprints/InventoryData_GameInstance_BP.Egg_Creature_Inventory` _asinventory_data_game_instance_bp))
          (bind _result_2 (`/Engine/EditorBlueprintResources/StandardMacros.IncrementInt` (`|GetArrayItem` _egg_creature_inventory _output_get))
            (:`  `
              (`KismetArrayLibrary.Array_Set` _egg_creature_inventory (`self.RNG`) _result_2)
              ;;[0.9522 0.3821 1] The same RNG is used to get the name of the mineral in the mineral string array (holds the mineral names).
              (set `/Game/Blueprints/InventoryData_GameInstance_BP.Egg_Creature_Grown` (`|GetArrayItem` (`/Game/Blueprints/InventoryData_GameInstance_BP.Egg_Creature` _asinventory_data_game_instance_bp) (`self.RNG`)) _asinventory_data_game_instance_bp)
              (`Widget.SetVisibility` (`/Game/Blueprints/UI/Main_Game_UI_AndTouch.Egg_Creature_Grown_Text` (`self.Main Game UIAnd Right Touch Ref`)) "Visible")
              (`KismetSystemLibrary.Delay` 3.0)
              (`Widget.SetVisibility` (`/Game/Blueprints/UI/Main_Game_UI_AndTouch.Egg_Creature_Grown_Text` (`self.Main Game UIAnd Right Touch Ref`)) "Hidden")))))
      (else
        ;[1 0 0] Tells player they have already incubated an egg here
        (`Widget.SetVisibility` _incubator_in_use_text "Visible")
        (`KismetSystemLibrary.Delay` 3.0)
        (`Widget.SetVisibility` _incubator_in_use_text "Hidden")))
    (else
      ;[0.3146 1 0.4649] If player has egg in inventory, remove one, set egg to incubated
      (bind _asinventory_data_game_instance_bp_2 (cast `/Game/Blueprints/InventoryData_GameInstance_BP` (`GameplayStatics.GetGameInstance`)))
      (bind _eggs (`/Game/Blueprints/InventoryData_GameInstance_BP.Eggs` _asinventory_data_game_instance_bp_2))
      (if (> _eggs 0)
        (set `/Game/Blueprints/InventoryData_GameInstance_BP.Eggs` (- _eggs 1) _asinventory_data_game_instance_bp_2)
        (set `self.EggIncubated` true)
        (`SceneComponent.SetVisibility` (`self.Egg`) true false)
        ;[0.5541 1 0.6092] Tell an egg has been incubated
        ;;[1 1 1] Show incubator timer
        (if (not (`SceneComponent.IsVisible` _in_world_widget))
          (`SceneComponent.SetVisibility` _in_world_widget true false)
          (`Widget.SetVisibility` (`/Game/Blueprints/UI/Main_Game_UI_AndTouch.EggHorizontalBox` (`self.Main Game UIAnd Right Touch Ref`)) "Visible")
          (`Widget.SetVisibility` (`/Game/Blueprints/UI/Main_Game_UI_AndTouch.Speed_up_button_1` (`self.Main Game UIAnd Right Touch Ref`)) "Visible")
          (`SceneComponent.SetVisibility` (`self.Highlight`) false false)
          (`Widget.SetVisibility` (`/Game/Blueprints/UI/Main_Game_UI_AndTouch.EggHorizontalBox` (`self.Main Game UIAnd Right Touch Ref`)) "Hidden")
          (bind (_direction _incubator_timer) (`Timeline|Incubator_Timer` :`NewTime` 599.900024 :!via `PlayFromStart` :!label _label_2)
            (:`Update`
              ;;[1 1 1] Stores the timer in the inventory data
              (set `/Game/Blueprints/InventoryData_GameInstance_BP.Incubator_Timer` _incubator_timer _as_inventory_data_game_instance_bp)
              ;;[1 1 1] Every tick check if the points used boolean is true. if it is, set it to false, set the timer to end. (Using points to speed up growth).
              (if (`/Game/Blueprints/UI/Main_Game_UI_AndTouch.Points_Used_0` _main_game_uiand_right_touch_ref)
                (set `/Game/Blueprints/UI/Main_Game_UI_AndTouch.Points_Used_0` false _main_game_uiand_right_touch_ref)
                (set `/Game/Blueprints/InventoryData_GameInstance_BP.Is_Egg_Ready` true _as_inventory_data_game_instance_bp)
                (goto _label_2 :!via `SetNewTime`)))
            (:`Finished`
              (set `/Game/Blueprints/InventoryData_GameInstance_BP.Is_Egg_Ready` true _as_inventory_data_game_instance_bp)
              (`SceneComponent.SetVisibility` (`self.Exclamation mark`) true false)
              (`SceneComponent.SetVisibility` (`self.Exclamation mark1`) true false)
              (`SceneComponent.SetVisibility` (`self.In_World_Widget`) false false)
              (`Widget.SetVisibility` (`/Game/Blueprints/UI/Main_Game_UI_AndTouch.Speed_up_button_1` (`self.Main Game UIAnd Right Touch Ref`)) "Hidden"))))
        (else
          ;[1 0 0] Tells player they have no eggs to incubate
          (`Widget.SetVisibility` _no_eggs_text "Visible")
          (`KismetSystemLibrary.Delay` 3.0)
          (`Widget.SetVisibility` _no_eggs_text "Hidden"))))))

(event `self.IncubatorHitbox.OnComponentEndOverlap`
  (params (OverlappedComponent :type "PrimitiveComponent Object Reference") (OtherActor :type "Actor Object Reference") (OtherComp :type "PrimitiveComponent Object Reference") (OtherBodyIndex :type Integer))
  ;[1 1 1] Make dialogue hitbox touchable, hide interactable hitbox
  (bind _asthird_person_character (cast `/Game/Blueprints/ThirdPersonCharacter` OtherActor))
  (`Widget.SetVisibility` (`/Game/Blueprints/UI/Main_Game_UI_AndTouch.Right_Touch_Button_Interactable_Seeds` (`/Game/Blueprints/ThirdPersonCharacter.MainGameUIAndRightTouch_Ref` _asthird_person_character)) "Hidden")
  (`Widget.SetVisibility` (`/Game/Blueprints/UI/Main_Game_UI_AndTouch.Eggs_Screen_Canvas` (`self.Main Game UIAnd Right Touch Ref`)) "Hidden")
  (`Widget.SetVisibility` (`/Game/Blueprints/UI/Main_Game_UI_AndTouch.Speed_Up_Growth_Canvas_1` (`/Game/Blueprints/ThirdPersonCharacter.MainGameUIAndRightTouch_Ref` _asthird_person_character)) "Hidden")
  (`Widget.SetVisibility` (`/Game/Blueprints/UI/Main_Game_UI_AndTouch.Right_Touch_Button_Interactables_Eggs` (`/Game/Blueprints/ThirdPersonCharacter.MainGameUIAndRightTouch_Ref` _asthird_person_character)) "Hidden")
  (`SceneComponent.SetVisibility` (`self.Highlight`) false false))

(fn `UserConstructionScript`)