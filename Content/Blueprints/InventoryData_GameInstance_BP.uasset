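; Game instance Blueprint that holds the player's progression data: EXP, level and skill points.
; CheckLevelUp performs one level-up per call when EXP reaches the threshold, setting a LevelUp flag, carrying surplus EXP over, raising the threshold linearly and granting a skill point.
; TotalEXP accumulates the full EXP value before that carry-over.
; A separate ThirdPersonCast event caches a reference to the player's ThirdPersonCharacter.
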(event `CheckLevelUp`
  (if (>= (`self.EXP`) (`self.LevelUpThreshold`))
    (set `self.Level_Up` true)
    ;[1 1 1] Increment level
    (bind _result (`/Engine/EditorBlueprintResources/StandardMacros.IncrementInt` (`self.Level`))
      (:`  `
        (set `self.Level` _result)
        ;[1 1 1] Set total EXP to be exp + total exp
        (set `self.TotalEXP` (+ (`self.EXP`) (`self.TotalEXP`)))
        ;[1 1 1] Reset EXP (for progression bars)
        (set `self.EXP` (* (- (`self.LevelUpThreshold`) (`self.EXP`)) -1.0))
        ;[1 1 1] Increase level up threshold
        (set `self.LevelUpThreshold` (+ (`self.LevelUpThreshold`) 2.0))
        ;[1 1 1] Increment skill points
        (set `self.Skill Points` (+ (`self.Skill Points`) 1.0))))))

(event `ThirdPersonCast`
  (bind _asthird_person_character (cast `/Game/Blueprints/ThirdPersonCharacter` (`GameplayStatics.GetPlayerCharacter` 0)))
  (set `self.As Third Person Character` _asthird_person_character))